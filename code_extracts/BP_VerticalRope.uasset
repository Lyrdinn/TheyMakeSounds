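; Placeable vertical rope artifact that the third-person character can attach to once instantiated.
; While aiming, a downward sphere trace positions the spline rope and end spheres; validity depends on rope budget and height order, shown by material and DoOnce-gated sounds.
; Instantiating applies the final material, morphs the anchor and fits a capsule between both ends.
; Capsule overlaps flag the character as near the rope, and Interaction attaches it unless already ziplining or on a rope.
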(event `self.ReceiveBeginPlay`
  (bind _splinerope (`self.SplineRope`))
  (`PrimitiveComponent.SetCollisionEnabled` (`self.CapsuleCollision`) "NoCollision")
  (`SceneComponent.K2_SetRelativeLocation` _splinerope (0.0 0.0 0.0) false false)
  (`PrimitiveComponent.SetMaterial` _splinerope 0 (`self.PreviewMaterial`))
  (`SkeletalMeshComponent.SetMorphTarget` (`self.SphereStart`) "GriiffOpen" 1.0 true)
  (`SkeletalMeshComponent.SetMorphTarget` (`self.SphereStart`) "TopFlat" 0.0 true))

(event `/Game/TheyMakeSound/Blueprints/Interfaces/BPI_Artifact.ShowHidePreview`
  (params (Show :type Boolean))
  (`SceneComponent.SetVisibility` (`self.SphereStart`) Show false)
  (`SceneComponent.SetVisibility` (`self.SplineRope`) Show false))

(event `/Game/TheyMakeSound/Blueprints/Interfaces/BPI_Artifact.SetCanInstantiate`
  (params (Rope :type "Float (double-precision)"))
  (bind (_returnvalue_x _returnvalue_y _returnvalue_z) (`KismetMathLibrary.BreakVector` (`SceneComponent.K2_GetComponentLocation` (`self.SphereStart`))))
  (bind (_returnvalue_x_2 _returnvalue_y_2 _returnvalue_z_2) (`KismetMathLibrary.BreakVector` (`SceneComponent.K2_GetComponentLocation` (`self.SphereEnd`))))
  (bind _ropelength (`self.GetLength`))
  (bind _output_get (set `self.CanInstantiate` (and (>= (* Rope 1000.0) _ropelength) (> _returnvalue_z _returnvalue_z_2))))
  ;[0.05098 0.05098 0.05098] Set Material based on if the player has enough rope or not
  (if _output_get
    (`PrimitiveComponent.SetMaterial` (`self.SplineRope`) 0 (`self.PreviewMat`))
    (`|ExecutionSequence`
      (:`then_0`
        (`/Engine/EditorBlueprintResources/StandardMacros.DoOnce` false :!label _label
          (:`Completed`
            (`AkGameObject.PostAssociatedAkEvent` :`self` (`self.AK_VertRopePreviewRight`)))))
      (:`then_1`
        (goto _label_2 :!via `Reset`)))
    (else
      (`PrimitiveComponent.SetMaterial` (`self.SplineRope`) 0 (`self.PreviewWrongMat`))
      (`|ExecutionSequence`
        (:`then_0`
          (`/Engine/EditorBlueprintResources/StandardMacros.DoOnce` false :!label _label_2
            (:`Completed`
              (`AkGameObject.PostAssociatedAkEvent` :`self` (`self.AK_VertRopePreviewWrong`)))))
        (:`then_1`
          (goto _label :!via `Reset`))))))

(event `/Game/TheyMakeSound/Blueprints/Interfaces/BPI_Artifact.MoveArtifactAim`
  (params (Charamesh :type "Vector Structure") (AimLocation :type "Vector Structure"))
  (bind _returnvalue (+ AimLocation (0.0 0.0 -30.0)))
  (bind (_offsetfromground_x _offsetfromground_y _offsetfromground_z) (`KismetMathLibrary.BreakVector` (`self.OffsetFromGround`)))
  (bind (_returnvalue_x _returnvalue_y _returnvalue_z) (`KismetMathLibrary.BreakVector` (`SceneComponent.K2_GetComponentLocation` (`self.SphereStart`))))
  (bind (_outhit _returnvalue_2) (`KismetSystemLibrary.SphereTraceSingleByProfile` :`Start` _returnvalue :`End` (+ _returnvalue (`KismetMathLibrary.MakeVector` 0.0 0.0 (* (`self.BaseVerticalRopeLength`) -1000.0))) :`ProfileName` "NoCollision" :`DrawTime` 0.0))
  (bind (_bblockinghit _binitialoverlap _time _distance _location) (`GameplayStatics.BreakHitResult` _outhit))
  (`SplineMeshComponent.SetEndPosition` (`self.SplineRope`) (- _location AimLocation (0.0 0.0 -100.0)) true)
  (`SceneComponent.K2_SetWorldLocation` (`self.SphereStart`) _returnvalue false false)
  (if _returnvalue_2
    (bind _output_get (set `self.OffsetFromGround` _location))
    (if (> _returnvalue_z (.z _output_get))
      (`|ExecutionSequence`
        (:`then_0`
          (`SceneComponent.K2_SetWorldLocation` (`self.SphereEnd`) (`KismetMathLibrary.MakeVector` _offsetfromground_x _offsetfromground_y (+ _offsetfromground_z 50.0)) false false)))
      (else
        (`SceneComponent.K2_SetWorldLocation` (`self.SphereEnd`) (`KismetMathLibrary.MakeVector` _offsetfromground_x _offsetfromground_y _offsetfromground_z) false false)))))

(event `/Game/TheyMakeSound/Blueprints/Interfaces/BPI_Artifact.InstantiateArtefact`
  (bind _returnvalue (- (`SceneComponent.K2_GetComponentLocation` (`self.SphereStart`)) (`SceneComponent.K2_GetComponentLocation` (`self.SphereEnd`))))
  (bind (_returnvalue_x _returnvalue_y _returnvalue_z) (`KismetMathLibrary.BreakVector` (/ _returnvalue 2.0)))
  (`PrimitiveComponent.SetMaterial` (`self.SplineRope`) 0 (`self.RenderMaterial`))
  ;[0.05098 0.05098 0.05098] Calculate capsule size and position
  (`SceneComponent.K2_SetWorldLocation` (`self.CapsuleCollision`) (- (`SceneComponent.K2_GetComponentLocation` (`self.SphereStart`)) (/ _returnvalue 2.0)) false false)
  (`CapsuleComponent.SetCapsuleHalfHeight` (`self.CapsuleCollision`) _returnvalue_z true)
  (`AkGameObject.PostAssociatedAkEvent` :`self` (`self.AK_VertRopeAnchor`))
  (`PrimitiveComponent.SetCollisionEnabled` (`self.CapsuleCollision`) "QueryAndPhysics")
  (`SkeletalMeshComponent.SetMorphTarget` (`self.SphereStart`) "GriiffOpen" 0.0 true)
  (`SkeletalMeshComponent.SetMorphTarget` (`self.SphereStart`) "TopFlat" 1.0 true))

(event `/Game/TheyMakeSound/Blueprints/Interfaces/BPI_Interaction.Interaction`
  (bind _asbp_third_person_character (cast `/Game/ThirdPerson/Blueprints/BP_ThirdPersonCharacter` (`GameplayStatics.GetPlayerCharacter` 0)))
  (if (not (or (`/Game/ThirdPerson/Blueprints/BP_ThirdPersonCharacter.Is Ziplining` _asbp_third_person_character) (`/Game/ThirdPerson/Blueprints/BP_ThirdPersonCharacter.Is Vertical` _asbp_third_person_character)))
    (set `/Game/ThirdPerson/Blueprints/BP_ThirdPersonCharacter.BP_Vertical` self _asbp_third_person_character)
    (set `/Game/ThirdPerson/Blueprints/BP_ThirdPersonCharacter.Is Vertical` true _asbp_third_person_character)
    (set `/Game/ThirdPerson/Blueprints/BP_ThirdPersonCharacter.Near Vertical` false _asbp_third_person_character)
    (`/Game/ThirdPerson/Blueprints/BP_ThirdPersonCharacter.On Interactable Entered/Exited` _asbp_third_person_character)))

(event `self.CapsuleCollision.OnComponentBeginOverlap`
  (params (OverlappedComponent :type "PrimitiveComponent Object Reference") (OtherActor :type "Actor Object Reference") (OtherComp :type "PrimitiveComponent Object Reference") (OtherBodyIndex :type Integer) (bFromSweep :type Boolean) (SweepResult :type "HitResult Structure (by ref)"))
  (bind _ascapsule_collision (cast `CapsuleComponent` OtherComp))
  (bind _asbp_third_person_character (cast `/Game/ThirdPerson/Blueprints/BP_ThirdPersonCharacter` (`ActorComponent.GetOwner` _ascapsule_collision)))
  (set `/Game/ThirdPerson/Blueprints/BP_ThirdPersonCharacter.Can Vertical` true _asbp_third_person_character)
  (if (not (`/Game/ThirdPerson/Blueprints/BP_ThirdPersonCharacter.Is Vertical` _asbp_third_person_character))
    (set `/Game/ThirdPerson/Blueprints/BP_ThirdPersonCharacter.Near Vertical` true _asbp_third_person_character)
    (`/Game/ThirdPerson/Blueprints/BP_ThirdPersonCharacter.On Interactable Entered/Exited` _asbp_third_person_character)))

(event `self.CapsuleCollision.OnComponentEndOverlap`
  (params (OverlappedComponent :type "PrimitiveComponent Object Reference") (OtherActor :type "Actor Object Reference") (OtherComp :type "PrimitiveComponent Object Reference") (OtherBodyIndex :type Integer))
  (bind _ascapsule_collision (cast `CapsuleComponent` OtherComp))
  (bind _asbp_third_person_character (cast `/Game/ThirdPerson/Blueprints/BP_ThirdPersonCharacter` (`ActorComponent.GetOwner` _ascapsule_collision)))
  (set `/Game/ThirdPerson/Blueprints/BP_ThirdPersonCharacter.Can Vertical` false _asbp_third_person_character)
  (set `/Game/ThirdPerson/Blueprints/BP_ThirdPersonCharacter.Near Vertical` false _asbp_third_person_character)
  (`/Game/ThirdPerson/Blueprints/BP_ThirdPersonCharacter.On Interactable Entered/Exited` _asbp_third_person_character))

(fn `GetCanInstantiate`
  (returns (NewParam :type Boolean))
  (return (and (`self.CanInstantiate`) (`SceneComponent.IsVisible` (`self.SplineRope`)))))

(fn `GetLength`
  (returns (RopeLength :type "Float (double-precision)"))
  (return (`KismetMathLibrary.Vector_Distance` (`SceneComponent.K2_GetComponentLocation` (`self.SphereStart`)) (`SceneComponent.K2_GetComponentLocation` (`self.SphereEnd`)))))

(fn `UserConstructionScript`)