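; Zipline actor the player aims and places, with a preview that shows whether placement is valid.
; Start sphere snaps above the character while the end interpolates to the aim point; the character validates rope and angle, driving preview materials, figure visibility and once-only Wwise cues.
; Instantiation reveals the cable and switches end-mesh morph targets.
; A capsule stretched between endpoints sets the character's zipline flags on overlap; Interaction is empty.
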(event `self.ReceiveBeginPlay`
  (`self.CalculateCapsuleLength`)
  (`SceneComponent.SetVisibility` (`self.PreviewCharacter`) false false)
  (for _index (range 3)
    (`PrimitiveComponent.SetMaterial` (`self.PreviewCharacter`) _index (`self.PreviewMaterialCharacter`))
    (if (not (`self.IsAlreadyInScene`))
      (`SkeletalMeshComponent.SetMorphTarget` (`self.SK_End`) "GriiffOpen" 1.0 true)
      (`SkeletalMeshComponent.SetMorphTarget` (`self.SK_Start`) "GriiffOpen" 1.0 true)
      (`SkeletalMeshComponent.SetMorphTarget` (`self.SK_End`) "TopFlat" 0.0 true)
      (`SkeletalMeshComponent.SetMorphTarget` (`self.SK_Start`) "TopFlat" 0.0 true))))

(event `/Game/TheyMakeSound/Blueprints/Interfaces/BPI_Artifact.ShowHidePreview`
  (params (Show :type Boolean))
  (`SceneComponent.SetVisibility` (`self.SphereStart`) Show false)
  (`SceneComponent.SetVisibility` (`self.SphereEnd`) Show false)
  (`SceneComponent.SetVisibility` (`self.ZiplinePreview`) Show false))

(event `/Game/TheyMakeSound/Blueprints/Interfaces/BPI_Artifact.SetCanInstantiate`
  (params (Rope :type "Float (double-precision)"))
  (bind _previewcharacter (`self.PreviewCharacter`))
  (bind (_returnvalue_roll _returnvalue_pitch _returnvalue_yaw) (`KismetMathLibrary.BreakRotator` (`KismetMathLibrary.FindLookAtRotation` (`SceneComponent.K2_GetComponentLocation` (`self.SphereStart`)) (`SceneComponent.K2_GetComponentLocation` (`self.SK_End`)))))
  (bind _returnvalue (`KismetMathLibrary.Vector_Distance` (`SceneComponent.K2_GetComponentLocation` (`self.SphereStart`)) (`SceneComponent.K2_GetComponentLocation` (`self.SphereEnd`))))
  (bind _returnvalue_2 (/ _returnvalue 100.0))
  (bind _asbp_third_person_character (cast `/Game/ThirdPerson/Blueprints/BP_ThirdPersonCharacter` (`GameplayStatics.GetPlayerPawn` 0)))
  (bind _ziplineangle (`self.GetZiplineDegree`))
  (bind _playermetrics (`/Game/ThirdPerson/Blueprints/BP_ThirdPersonCharacter.PlayerMetrics` _asbp_third_person_character))
  (bind _output_get (set `self.CanInstantiateZipline` (and (>= _ziplineangle 2.0) (>= (* Rope 1000.0) _returnvalue) (>= _returnvalue_2 (`PlayerMetrics.ZiplineMinDist` _playermetrics)) (<= _returnvalue_2 (`PlayerMetrics.ZiplineMaxDist` _playermetrics)))))
  (`SceneComponent.K2_SetWorldRotation` _previewcharacter (`KismetMathLibrary.MakeRotator` 0.0 0.0 (+ _returnvalue_yaw -90.0)) false false)
  (`SceneComponent.SetVisibility` _previewcharacter _output_get false)
  ;[0.05208 0.05208 0.05208] Set Material based on if the player has enough rope or not
  (if (`self.CanInstantiateZipline`)
    (`PrimitiveComponent.SetMaterial` (`self.ZiplinePreview`) 0 (`self.PreviewMaterial`))
    (`|ExecutionSequence`
      (:`then_1`
        (`/Engine/EditorBlueprintResources/StandardMacros.DoOnce` false :!label _label
          (:`Completed`
            (`AkGameObject.PostAssociatedAkEvent` :`self` (`self.AK_ZiplinePreviewRight`)))))
      (:`then_2`
        (goto _label_2 :!via `Reset`)))
    (else
      (`PrimitiveComponent.SetMaterial` (`self.ZiplinePreview`) 0 (`self.PreviewWrongMat`))
      (`|ExecutionSequence`
        (:`then_1`
          (`/Engine/EditorBlueprintResources/StandardMacros.DoOnce` false :!label _label_2
            (:`Completed`
              (`AkGameObject.PostAssociatedAkEvent` :`self` (`self.AK_ZiplinePreviewWrong`)))))
        (:`then_2`
          (goto _label :!via `Reset`))))))

(event `/Game/TheyMakeSound/Blueprints/Interfaces/BPI_Artifact.MoveArtifactAim`
  (params (Charamesh :type "Vector Structure") (AimLocation :type "Vector Structure"))
  (bind _sk_end (`self.SK_End`))
  (bind _sphereend (`self.SphereEnd`))
  (bind (_returnvalue_roll _returnvalue_pitch _returnvalue_yaw) (`KismetMathLibrary.BreakRotator` (`KismetMathLibrary.FindLookAtRotation` (`SceneComponent.K2_GetComponentLocation` _sk_end) (`SceneComponent.K2_GetComponentLocation` (`self.SK_Start`)))))
  (bind (_returnvalue_roll_2 _returnvalue_pitch_2 _returnvalue_yaw_2) (`KismetMathLibrary.BreakRotator` (`KismetMathLibrary.FindLookAtRotation` (`SceneComponent.K2_GetComponentLocation` (`self.SK_Start`)) (`SceneComponent.K2_GetComponentLocation` (`self.SK_End`)))))
  (`SceneComponent.K2_SetWorldLocation` (`self.SphereStart`) (+ Charamesh (0.0 0.0 200.0)) false false)
  (`SceneComponent.K2_SetWorldLocation` _sphereend (`KismetMathLibrary.VInterpTo` (`SceneComponent.K2_GetComponentLocation` _sphereend) (+ AimLocation (-30.0 0.0 250.0)) (`GameplayStatics.GetWorldDeltaSeconds`) 10.0) false false)
  (`SceneComponent.K2_SetWorldRotation` (`self.SK_Start`) (`KismetMathLibrary.MakeRotator` _returnvalue_roll_2 (+ _returnvalue_pitch_2 -90.0) _returnvalue_yaw_2) false false)
  (`SceneComponent.K2_SetWorldRotation` _sk_end (`KismetMathLibrary.MakeRotator` _returnvalue_roll (+ _returnvalue_pitch 90.0) _returnvalue_yaw) false false))

(event `/Game/TheyMakeSound/Blueprints/Interfaces/BPI_Artifact.InstantiateArtefact`
  (bind _zipline (`self.Zipline`))
  (`SceneComponent.SetVisibility` (`self.ZiplinePreview`) false false)
  (set `CableComponent.bAttachEnd` true _zipline)
  (`CableComponent.SetAttachEndToComponent` _zipline (`self.SphereEnd`) "None")
  (`SceneComponent.SetVisibility` (`self.Zipline`) true false)
  (`self.CalculateCapsuleLength`)
  (`AkGameObject.PostAssociatedAkEvent` :`self` (`self.AK_ZiplineMaterialize`))
  (`SkeletalMeshComponent.SetMorphTarget` (`self.SK_End`) "GriiffOpen" 0.0 true)
  (`SkeletalMeshComponent.SetMorphTarget` (`self.SK_Start`) "GriiffOpen" 0.0 true)
  (`SkeletalMeshComponent.SetMorphTarget` (`self.SK_End`) "TopFlat" 1.0 true)
  (`SkeletalMeshComponent.SetMorphTarget` (`self.SK_Start`) "TopFlat" 1.0 true)
  (`ActorComponent.K2_DestroyComponent` (`self.PreviewCharacter`)))

(event `self.CapsuleCollision.OnComponentBeginOverlap`
  (params (OverlappedComponent :type "PrimitiveComponent Object Reference") (OtherActor :type "Actor Object Reference") (OtherComp :type "PrimitiveComponent Object Reference") (OtherBodyIndex :type Integer) (bFromSweep :type Boolean) (SweepResult :type "HitResult Structure (by ref)"))
  (bind _ascapsule_collision (cast `CapsuleComponent` OtherComp))
  (bind _asbp_third_person_character (cast `/Game/ThirdPerson/Blueprints/BP_ThirdPersonCharacter` (`ActorComponent.GetOwner` _ascapsule_collision)))
  (set `/Game/ThirdPerson/Blueprints/BP_ThirdPersonCharacter.Can Zipline` true _asbp_third_person_character)
  (if (not (`/Game/ThirdPerson/Blueprints/BP_ThirdPersonCharacter.Is Ziplining` _asbp_third_person_character))
    (set `/Game/ThirdPerson/Blueprints/BP_ThirdPersonCharacter.Near Zipline` true _asbp_third_person_character)
    (`/Game/ThirdPerson/Blueprints/BP_ThirdPersonCharacter.On Interactable Entered/Exited` _asbp_third_person_character)))

(event `self.CapsuleCollision.OnComponentEndOverlap`
  (params (OverlappedComponent :type "PrimitiveComponent Object Reference") (OtherActor :type "Actor Object Reference") (OtherComp :type "PrimitiveComponent Object Reference") (OtherBodyIndex :type Integer))
  (bind _ascapsule_collision (cast `CapsuleComponent` OtherComp))
  (bind _asbp_third_person_character (cast `/Game/ThirdPerson/Blueprints/BP_ThirdPersonCharacter` (`ActorComponent.GetOwner` _ascapsule_collision)))
  (set `/Game/ThirdPerson/Blueprints/BP_ThirdPersonCharacter.Can Zipline` false _asbp_third_person_character)
  (set `/Game/ThirdPerson/Blueprints/BP_ThirdPersonCharacter.Near Zipline` false _asbp_third_person_character)
  (`/Game/ThirdPerson/Blueprints/BP_ThirdPersonCharacter.On Interactable Entered/Exited` _asbp_third_person_character))

(event `/Game/TheyMakeSound/Blueprints/Interfaces/BPI_Interaction.Interaction`)

(fn `CalculateCapsuleLength`
  (bind _returnvalue (`SceneComponent.K2_GetComponentLocation` (`self.SphereStart`)))
  (bind _returnvalue_2 (`SceneComponent.K2_GetComponentLocation` (`self.SphereEnd`)))
  (bind (_returnvalue_roll _returnvalue_pitch _returnvalue_yaw) (`KismetMathLibrary.BreakRotator` (`KismetMathLibrary.FindLookAtRotation` (`SceneComponent.K2_GetComponentLocation` (`self.SphereStart`)) (`SceneComponent.K2_GetComponentLocation` (`self.SphereEnd`)))))
  (`SceneComponent.K2_SetWorldLocation` (`self.CapsuleCollision`) (- (`SceneComponent.K2_GetComponentLocation` (`self.SphereStart`)) (/ (- _returnvalue _returnvalue_2) 2.0)) false false)
  (`CapsuleComponent.SetCapsuleHalfHeight` (`self.CapsuleCollision`) (/ (`KismetMathLibrary.Vector_Distance` _returnvalue _returnvalue_2) 2.0) true)
  (`SceneComponent.K2_SetWorldRotation` (`self.CapsuleCollision`) (`KismetMathLibrary.MakeRotator` 0.0 (+ _returnvalue_pitch 90.0) _returnvalue_yaw) false false)
  (`ActorComponent.SetActive` (`self.CapsuleCollision`) true false))

(fn `GetCanInstantiate`
  (returns (NewParam :type Boolean))
  (return (and (`self.CanInstantiateZipline`) (`SceneComponent.IsVisible` (`self.ZiplinePreview`)))))

(fn `GetLength`
  (returns (RopeLength :type "Float (double-precision)"))
  (return (`KismetMathLibrary.Vector_Distance` (`SceneComponent.K2_GetComponentLocation` (`self.SphereStart`)) (`SceneComponent.K2_GetComponentLocation` (`self.SphereEnd`)))))

(fn `GetZiplineDegree`
  (returns (ZiplineAngle :type "Float (double-precision)"))
  (bind (_returnvalue_roll _returnvalue_pitch) (`KismetMathLibrary.BreakRotator` (`KismetMathLibrary.FindLookAtRotation` (`SceneComponent.K2_GetComponentLocation` (`self.SphereEnd`)) (`SceneComponent.K2_GetComponentLocation` (`self.SphereStart`)))))
  (return _returnvalue_pitch))

(fn `GetZiplineLength`
  (returns (Length :type "Float (double-precision)"))
  (return (`KismetMathLibrary.Vector_Distance` (`SceneComponent.GetSocketLocation` (`self.SphereStart`) "None") (`SceneComponent.GetSocketLocation` (`self.SphereEnd`) "None"))))

(fn `UserConstructionScript`)